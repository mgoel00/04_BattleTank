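; Enemy tank Blueprint that wires up its aiming, movement and health bar when play begins.
; BeginPlay passes the barrel and turret to the TankAiming component and the left and right tracks to TankMovement.
; It then casts the HealthBar component's user widget to the HealthBar class and sets its MyTank reference to this tank.
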(event EventBeginPlay
  (Class|TankAimingComponent|Initialise (Variables|Default|GetTankAiming) (Variables|Default|GetBarrel) (Variables|Default|GetTurret))
  (Class|TankMovementComponent|Initialise (Variables|Default|GetTankMovement) (Variables|Default|GetLeft%20Track) (Variables|Default|GetRight%20Track))
  (CallFunction|InitialiseHealthBarWidget))

(fn ConstructionScript)

(fn InitialiseHealthBarWidget
  (bind _ashealth_bar (Utilities|Casting|CastToHealthBar (UserInterface|GetUserWidgetObject (Variables|Default|GetHealth%20Bar))))
  (Variables|/Game/UI/HealthBar.HealthBar_C|SetMyTank _ashealth_bar self)
  (return))